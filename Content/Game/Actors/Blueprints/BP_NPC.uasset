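; Side-scrolling 2D enemy NPC that chases and punches the player's BP_Owlet.
; Tick walks it along X while the player is inside the detection Sphere, and attacks once the player enters AttackRange.
; Attacks use delayed hit-or-whiff checks and a DoOnce reset by a cooldown timer.
; Impact decrements health until death destroys the actor; a priority-based function picks flipbooks, and sprite yaw follows movement direction.
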(event `self.ReceiveBeginPlay`
  ;[0.8042 0.3277 1] Initialize
  (`ActorComponent.SetIsReplicated` (`self.Sprite`) true)
  (set `self.CurrentHealth` 4))

(event `self.OnLanded`
  (params (Hit :type "HitResult Structure (by ref)"))
  ;[1 1 1] Handle Animation
  (set `self.Is Falling` true))

(event `UpdateAnimation`
  ;[1 1 1] Handle Animation
  (set `self.IsMoving` (> (`KismetMathLibrary.VSize` (`self.GetVelocity`)) 0.0))
  (set `self.Is Falling` (`NavMovementComponent.IsFalling` (`self.CharacterMovement`)))
  (bind _outputflipbook (`self.Animation State Machine` (`self.Is Falling`) (`self.IsMoving`) (`self.Is Running`)))
  (`PaperFlipbookComponent.SetFlipbook` (`self.Sprite`) _outputflipbook))

(event `Attack`
  ;[1 1 1] Attack Animation/connect check
  (`/Engine/EditorBlueprintResources/StandardMacros.DoOnce` false :!label _label
    (:`Completed`
      (`|ExecutionSequence`
        (:`then_0`
          (set `self.Is Attacking` true)
          (`self.UpdateAnimation`) ; Play attack animation
          (`KismetSystemLibrary.Delay` 0.3) ; Wait for animation to play
          (if (`self.AttackOverlap`)
            (`GameplayStatics.PlaySound2D` "/Game/Game/Assets/Sounds/punch.punch" 1.0 1.0 0.0 null null)
            (bind _asbp_owlet (cast `/Game/Game/Actors/Blueprints/BP_Owlet` (`GameplayStatics.GetPlayerCharacter` 0)))
            (`/Game/Game/Actors/Blueprints/BP_Owlet.Hit` _asbp_owlet)
            (`KismetSystemLibrary.Delay` 0.3)
            (set `self.Is Attacking` false)
            (else
              (`GameplayStatics.PlaySound2D` "/Game/Game/Assets/Sounds/whiff.whiff" 1.0 1.0 0.0 null null)
              (`KismetSystemLibrary.Delay` 0.4)
              (set `self.Is Attacking` false))))
        (:`then_1`
          _))
      (`KismetSystemLibrary.K2_SetTimerDelegate` (delegate `AttackCooldown`) 1.0))))

(event `AttackCooldown`
  ;[1 1 1] Attack Animation/connect check
  (goto _label :!via `Reset`))

(event `self.ReceiveTick`
  (params (DeltaSeconds :type "Float (single-precision)"))
  (bind _returnvalue_x (`KismetMathLibrary.BreakVector` (`SceneComponent.K2_GetComponentLocation` (`self.CapsuleComponent`))))
  ;[1 1 1] Tick - Updates animation
  (if (`self.IsDead`)
    _
    (elif (`self.Overlapping`)
      (if (`self.AttackOverlap`)
        (`self.Attack`)
        (else
          ;[1 1 1] Movement
          (bind _asbp_owlet (cast `/Game/Game/Actors/Blueprints/BP_Owlet` (`GameplayStatics.GetPlayerCharacter` 0)))
          (bind _returnvalue_x_2 (`KismetMathLibrary.BreakVector` (`SceneComponent.K2_GetComponentLocation` (`Character.CapsuleComponent` _asbp_owlet))))
          (bind _returnvalue (- _returnvalue_x_2 _returnvalue_x))
          (if (<= _returnvalue 0.0)
            (set `self.IsLookingRight` false)
            (else
              (set `self.IsLookingRight` true)))
          (`self.AddMovementInput` (1.0 0.0 0.0) _returnvalue)))))
  (`self.UpdateAnimation`)
  (if (`self.IsDead`)
    (`KismetSystemLibrary.Delay` 0.8)
    (`self.K2_DestroyActor`)
    (else
      (`/Engine/EditorBlueprintResources/StandardMacros.CompareFloat` (.x (`MovementComponent.Velocity` (`self.GetMovementComponent`)))
        (:`>`
          (`/Engine/EditorBlueprintResources/StandardMacros.IsValid` null :!label _label_2
            (:`Is Valid`
              _)
            (:`Is Not Valid`
              _))
          (`SceneComponent.K2_SetWorldRotation` (`self.Sprite`) (`KismetMathLibrary.MakeRotator` 0.0) false false)
          (`SceneComponent.K2_SetWorldRotation` (`Actor.RootComponent` (`self.GetController`)) (`KismetMathLibrary.MakeRotator` 0.0) false false))
        (:`==`
          (if (`self.IsLookingRight`)
            (goto _label_2)
            (else
              (`/Engine/EditorBlueprintResources/StandardMacros.IsValid` null :!label _label_3
                (:`Is Valid`
                  _)
                (:`Is Not Valid`
                  _))
              (`SceneComponent.K2_SetWorldRotation` (`self.Sprite`) (`KismetMathLibrary.MakeRotator` 0.0 0.0 180.0) false false)
              (`SceneComponent.K2_SetWorldRotation` (`Actor.RootComponent` (`self.GetController`)) (`KismetMathLibrary.MakeRotator` 0.0 0.0 180.0) false false))))
        (:`<`
          (goto _label_3))))))

(event `self.Sphere.OnComponentBeginOverlap`
  (params (OverlappedComponent :type "PrimitiveComponent Object Reference") (OtherActor :type "Actor Object Reference") (OtherComp :type "PrimitiveComponent Object Reference") (OtherBodyIndex :type Integer) (bFromSweep :type Boolean) (SweepResult :type "HitResult Structure (by ref)"))
  ;[1 1 1] Handle Overlaps
  (cast `/Game/Game/Actors/Blueprints/BP_Owlet` OtherActor)
  (set `self.Overlapping` true))

(event `self.Sphere.OnComponentEndOverlap`
  (params (OverlappedComponent :type "PrimitiveComponent Object Reference") (OtherActor :type "Actor Object Reference") (OtherComp :type "PrimitiveComponent Object Reference") (OtherBodyIndex :type Integer))
  ;[1 1 1] Handle Overlaps
  (cast `/Game/Game/Actors/Blueprints/BP_Owlet` OtherActor)
  (set `self.Overlapping` false))

(event `self.AttackRange.OnComponentBeginOverlap`
  (params (OverlappedComponent :type "PrimitiveComponent Object Reference") (OtherActor :type "Actor Object Reference") (OtherComp :type "PrimitiveComponent Object Reference") (OtherBodyIndex :type Integer) (bFromSweep :type Boolean) (SweepResult :type "HitResult Structure (by ref)"))
  ;[1 1 1] Handle Overlaps
  (cast `/Game/Game/Actors/Blueprints/BP_Owlet` OtherActor)
  (set `self.AttackOverlap` true))

(event `self.AttackRange.OnComponentEndOverlap`
  (params (OverlappedComponent :type "PrimitiveComponent Object Reference") (OtherActor :type "Actor Object Reference") (OtherComp :type "PrimitiveComponent Object Reference") (OtherBodyIndex :type Integer))
  ;[1 1 1] Handle Overlaps
  (cast `/Game/Game/Actors/Blueprints/BP_Owlet` OtherActor)
  (set `self.AttackOverlap` false))

(event `Impact`
  ;[0.25 0.25 0.25] Damage System
  (bind _returnvalue (`MyBlueprintFunctionLibrary.RemoveHealth` (`self.CurrentHealth`) 1))
  (bind _output_get (set `self.CurrentHealth` _returnvalue))
  (set `self.IsDead` (<= _output_get 0)))

(fn `Animation State Machine`
  (params (IsFalling :type Boolean) (IsMoving :type Boolean) (IsRunning :type Boolean))
  (returns (OutputFlipbook :type "PaperFlipbook Object Reference"))
  (locals (`Animation State` :type "/Game/Game/Actors/Data/Character_States Enum") (IsFallingLocal :type Boolean) (IsMovingLocal :type Boolean) (IsRunningLocal :type Boolean) (IsAttackingLocal :type Boolean) (IsDeadLocal :type Boolean))
  ;[1 1 1] State Machine
  (set `local.IsDeadLocal` (`self.IsDead`))
  (set `local.IsFallingLocal` IsFalling)
  (set `local.IsMovingLocal` IsMoving)
  (set `local.IsRunningLocal` IsRunning)
  (set `local.IsAttackingLocal` (`self.Is Attacking`))
  (if (`local.IsDeadLocal`)
    (set `local.Animation State` "NewEnumerator7")
    (elif (`local.IsAttackingLocal`)
      (set `local.Animation State` "NewEnumerator5")
      (elif (`local.IsFallingLocal`)
        (set `local.Animation State` "NewEnumerator3")
        (elif (`local.IsMovingLocal`)
          (if (`local.IsRunningLocal`)
            (set `local.Animation State` "NewEnumerator1")
            (else
              (set `local.Animation State` "NewEnumerator2")))
          (else
            (set `local.Animation State` "NewEnumerator0"))))))
  (return (select `/Game/Game/Actors/Data/Character_States` (`local.Animation State`) :`NewEnumerator0` (`self.IdleFlipbook`) :`NewEnumerator2` (`self.WalkFlipbook`) :`NewEnumerator1` (`self.RunFlipbook`) :`NewEnumerator3` (`self.JumpFlipbook`) :`NewEnumerator5` (`self.AttackFlipbook`) :`NewEnumerator7` (`self.DeadFlipbook`))))

(fn `UserConstructionScript`)