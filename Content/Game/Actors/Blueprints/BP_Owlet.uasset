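; BP_Owlet is the playable 2D side-scroller character, with walk, run, jump, projectile throwing, hearts-based health, and pause and death menus.
; Input and Hit/HeartCollect events update state flags, health and the HUD.
; Tick feeds those flags into a priority-ordered function that selects the sprite's flipbook, and flips facing through control rotation.
; On death, Tick instead waits for the animation, then pauses and shows the death widget.
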(event `self.ReceiveBeginPlay`
  ;[0.8042 0.3277 1] Initialize
  (`ActorComponent.SetIsReplicated` (`self.Sprite`) true)
  ;[1 1 1] Show HUD
  (bind _returnvalue (`|CreateWidget` "/Game/Game/Levels/GameLevels/Widgets/MainHUD.MainHUD_C" (`GameplayStatics.GetPlayerController` 0)))
  (bind _output_get (set `self.MainHUDRef` _returnvalue))
  (`UserWidget.AddToViewport` _output_get 0))

(event `UpdateAnimation`
  ;[1 1 1] Handle Animation
  (set `self.IsMoving` (> (`KismetMathLibrary.VSize` (`self.GetVelocity`)) 0.0))
  (set `self.Is Falling` (`NavMovementComponent.IsFalling` (`self.CharacterMovement`)))
  (bind _outputflipbook (`self.Animation State Machine`))
  (`PaperFlipbookComponent.SetFlipbook` (`self.Sprite`) _outputflipbook))

(event `InputAction|Jump`
  (params (Key :type "Key Structure"))
  ;[1 1 1] Handle Jump
  (:`Pressed`
    (`self.Jump` :!label _label)
    (set `self.State` "NewEnumerator3"))
  (:`Released`
    (`self.StopJumping` :!label _label_2)))

(event `InputAxis|MoveRight`
  (params (AxisValue :type "Float (single-precision)"))
  ;[1 1 1] Handle movement
  (if (not (or (`self.Is Throw`) (`self.IsPunching`)))
    (if (> AxisValue 0.0)
      (set `self.bisMovingRight` true)
      (elif (< AxisValue 0.0)
        (set `self.bisMovingRight` false)))
    (`self.AddMovementInput` (1.0 0.0 0.0) AxisValue)))

(event `InputTouch`
  (params (Location :type "Vector Structure") (FingerIndex :type "ETouchIndex Enum"))
  ;[1 1 1] Handle Jump
  (:`Pressed`
    (goto _label))
  (:`Released`
    (goto _label_2)))

(event `self.OnLanded`
  (params (Hit :type "HitResult Structure (by ref)"))
  ;[1 1 1] Handle Jump
  (bind _returnvalue (`|SpawnActorFromClass` "/Game/Game/Actors/Blueprints/BP_Jump_Puff.BP_Jump_Puff_C" (`KismetMathLibrary.MakeTransform` (+ (`self.K2_GetActorLocation`) (1.0 0.0 -6.0))) "Undefined" "OverrideRootScale" null null))
  (`self.SetLifeSpan` _returnvalue 0.6)
  (set `self.Puff` _returnvalue)
  (set `self.State` "NewEnumerator0"))

(event `ThrowEvent`
  ;[1 1 1] Throw Projectile
  (`KismetSystemLibrary.Delay` 0.3)
  (`|SpawnActorFromClass` "/Game/Game/Actors/Blueprints/BP_Projectile.BP_Projectile_C" (`SceneComponent.K2_GetComponentToWorld` (`self.ProjectileSpawn`)) "AlwaysSpawn" "OverrideRootScale" null null)
  (`|ExecutionSequence`
    (:`then_0`
      (`GameplayStatics.PlaySound2D` "/Game/Game/Assets/Sounds/whoosh.whoosh" 1.0 1.0 0.0 null null))
    (:`then_1`
      _))
  (`KismetSystemLibrary.Delay` 0.1)
  (set `self.Is Throw` false))

(event `Key|LeftShift`
  (params (Key :type "Key Structure"))
  (bind _charactermovement (`self.CharacterMovement`))
  ;[1 1 1] Handle Run Input
  (:`Pressed`
    (set `self.Is Running` true)
    (set `CharacterMovementComponent.MaxWalkSpeed` 215.0 _charactermovement))
  (:`Released`
    (set `self.Is Running` false)
    (set `CharacterMovementComponent.MaxWalkSpeed` 100.0 _charactermovement)))

(event `InputAction|Throw`
  (params (Key :type "Key Structure"))
  ;[1 1 1] Throw Projectile
  (:`Pressed`
    (if (not (`self.Is Falling`))
      (set `self.Is Throw` true)
      (`self.ThrowEvent`))))

(event `self.ReceiveTick`
  (params (DeltaSeconds :type "Float (single-precision)"))
  (bind _returnvalue (`self.GetController`))
  (bind _returnvalue_2 (`self.GetController`))
  ;[1 1 1] Tick - Updates animation
  (`self.UpdateAnimation`)
  (if (`self.IsDead`)
    ;[1 1 1] Death Screen
    (`KismetSystemLibrary.Delay` 0.8) ; Allow death animation to play out
    (`GameplayStatics.SetGamePaused` true)
    (bind _returnvalue_3 (`|CreateWidget` "/Game/Game/Levels/GameLevels/Widgets/DeathWidget.DeathWidget_C"))
    (bind _output_get (set `self.Death_Menu_Ref` _returnvalue_3))
    (bind _returnvalue_4 (`AddComponent|NODE_AddWidgetInteractionComponent-0`))
    (`UserWidget.AddToViewport` _output_get 0)
    (set `PlayerController.bShowMouseCursor` true (`GameplayStatics.GetPlayerController` 0))
    (`WidgetInteractionComponent.SetFocus` _returnvalue_4 _output_get)
    (else
      (`/Engine/EditorBlueprintResources/StandardMacros.CompareFloat` (.x (`MovementComponent.Velocity` (`self.GetMovementComponent`)))
        (:`>`
          (`/Engine/EditorBlueprintResources/StandardMacros.IsValid` _returnvalue_2 :!label _label_3
            (:`Is Valid`
              (`Controller.SetControlRotation` _returnvalue_2 (`KismetMathLibrary.MakeRotator` 0.0)))))
        (:`==`
          (if (`self.bisMovingRight`)
            (goto _label_3)
            (else
              (`/Engine/EditorBlueprintResources/StandardMacros.IsValid` _returnvalue :!label _label_4
                (:`Is Valid`
                  (`Controller.SetControlRotation` _returnvalue (`KismetMathLibrary.MakeRotator` 0.0 0.0 180.0)))))))
        (:`<`
          (goto _label_4))))))

(event `Hit`
  (bind _health (`self.Health`))
  ;[1 1 1] Damage System
  (if (> _health 0)
    (bind _output_get (set `self.Health` (`KismetMathLibrary.Clamp` (- _health 1) 0 3)))
    (`/Game/Game/Levels/GameLevels/Widgets/MainHUD.Remove Heart` (`self.MainHUDRef`) _output_get)
    (set `self.IsFull` false)
    (if (== _output_get 0)
      (set `self.IsDead` true))))

(event `InputAction|Pause` :paused true
  (params (Key :type "Key Structure"))
  (bind _returnvalue (`GameplayStatics.GetPlayerController` 0))
  (bind _pause_menu_ref (`self.Pause_Menu_Ref`))
  ;[1 1 1] Pause System
  (:`Pressed`
    (`/Engine/EditorBlueprintResources/StandardMacros.IsValid` (`self.Pause_Menu_Ref`)
      (:`Is Valid`
        _)
      (:`Is Not Valid`
        (bind _returnvalue_2 (`|CreateWidget` "/Game/Game/Levels/Pause_Menu/PauseWidget.PauseWidget_C"))
        (bind _output_get (set `self.Pause_Menu_Ref` _returnvalue_2))))
    (if (`GameplayStatics.IsGamePaused`)
      (`Widget.RemoveFromParent` _pause_menu_ref)
      (`GameplayStatics.SetGamePaused` false)
      (set `PlayerController.bShowMouseCursor` false _returnvalue)
      (`WidgetBlueprintLibrary.SetInputMode_GameOnly` _returnvalue)
      (else
        (`UserWidget.AddToViewport` _output_get 0)
        (`GameplayStatics.SetGamePaused` true)
        (set `PlayerController.bShowMouseCursor` true _returnvalue)
        (`WidgetBlueprintLibrary.SetInputMode_GameAndUIEx` _returnvalue _pause_menu_ref "LockInFullscreen" false)))))

(event `HeartCollect`
  (bind _health (`self.Health`))
  ;[1 1 1] Gain Health System
  (if (!= _health (`self.MaxHealth`))
    (set `self.Health` (`KismetMathLibrary.Clamp` (+ _health 1) 0 3))
    (if (== (`self.Health`) (`self.MaxHealth`))
      (set `self.IsFull` true)
      (`/Game/Game/Levels/GameLevels/Widgets/MainHUD.Add Heart` (`self.MainHUDRef`) :!label _label_5)
      (elif (not (`self.IsFull`))
        (goto _label_5)))))

(fn `Animation State Machine`
  (returns (OutputFlipbook :type "PaperFlipbook Object Reference"))
  (locals (`Animation State` :type "/Game/Game/Actors/Data/Character_States Enum") (IsFallingLocal :type Boolean) (IsMovingLocal :type Boolean) (IsRunningLocal :type Boolean) (IsThrowingLocal :type Boolean) (IsPunchingLocal :type Boolean) (IsDeadLocal :type Boolean))
  ;[1 1 1] State Machine
  (set `local.IsDeadLocal` (`self.IsDead`))
  (set `local.IsPunchingLocal` (`self.IsPunching`))
  (set `local.IsThrowingLocal` (`self.Is Throw`))
  (set `local.IsPunchingLocal` (`self.IsPunching`))
  (set `local.IsFallingLocal` (`self.Is Falling`))
  (set `local.IsMovingLocal` (`self.IsMoving`))
  (set `local.IsRunningLocal` (`self.Is Running`))
  (if (`local.IsDeadLocal`)
    (set `local.Animation State` "NewEnumerator7")
    (elif (`local.IsPunchingLocal`)
      (set `local.Animation State` "NewEnumerator5")
      (elif (`local.IsThrowingLocal`)
        (set `local.Animation State` "NewEnumerator6")
        (elif (`local.IsFallingLocal`)
          (set `local.Animation State` "NewEnumerator3")
          (elif (`local.IsMovingLocal`)
            (if (`local.IsRunningLocal`)
              (set `local.Animation State` "NewEnumerator1")
              (else
                (set `local.Animation State` "NewEnumerator2")))
            (else
              (set `local.Animation State` "NewEnumerator0")))))))
  (return (select `/Game/Game/Actors/Data/Character_States` (`local.Animation State`) :`NewEnumerator0` (`self.IdleFlipbook`) :`NewEnumerator2` (`self.WalkFlipbook`) :`NewEnumerator1` (`self.RunFlipbook`) :`NewEnumerator3` (`self.JumpFlipbook`) :`NewEnumerator5` (`self.PunchFlipbook`) :`NewEnumerator6` (`self.ThrowFlipbook`) :`NewEnumerator7` (`self.DeadFlipbook`))))

(fn `UserConstructionScript`)