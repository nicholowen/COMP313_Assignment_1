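; NPC is a 2D Paper2D character that chases the player's BP_Owlet horizontally and switches to attacking once it enters attack range.
; Sphere and AttackRange overlaps set flags that Tick uses for movement, attacking and left/right facing; the attack flag never resets.
; A state-machine function selects the sprite flipbook, with Attack left unassigned.
; The animation update also spawns a short-lived BP_ChestInteract while overlapping the first BP_Chest found.
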(event `self.ReceiveBeginPlay`
  ;[0.8042 0.3277 1] Initialize
  (`ActorComponent.SetIsReplicated` (`self.Sprite`) true))

(event `UpdateAnimation`
  ;[1 1 1] Handle Animation
  (set `self.IsMoving` (> (`KismetMathLibrary.VSize` (`self.GetVelocity`)) 0.0))
  (set `self.Is Falling` (`NavMovementComponent.IsFalling` (`self.CharacterMovement`)))
  (bind _outputflipbook (`self.Animation State Machine` (`self.Is Falling`) (`self.IsMoving`) (`self.Is Running`)))
  (`PaperFlipbookComponent.SetFlipbook` (`self.Sprite`) _outputflipbook)
  ;[1 1 1] Handle Interaction Collisions
  (`PrimitiveComponent.SetCollisionEnabled` (`self.Sprite`) "QueryOnly")
  (bind _returnvalue (`GameplayStatics.GetActorOfClass` "/Game/Game/Blueprints/BP_Chest.BP_Chest_C"))
  (if (`self.IsOverlappingActor` (`ActorComponent.GetOwner` (`self.Sprite`)) _returnvalue)
    (bind _returnvalue_2 (`|SpawnActorFromClass` "/Game/Game/Blueprints/BP_ChestInteract.BP_ChestInteract_C" (`KismetMathLibrary.MakeTransform` (+ (`self.K2_GetActorLocation`) (0.0 0.0 30.0))) "Undefined" "OverrideRootScale" null null))
    (`self.SetLifeSpan` _returnvalue_2 0.01)
    (set `self.Chest` _returnvalue_2)))

(event `self.ReceiveTick`
  (params (DeltaSeconds :type "Float (single-precision)"))
  (bind _returnvalue (`self.GetController`))
  (bind _returnvalue_2 (`self.GetController`))
  (bind _returnvalue_x (`KismetMathLibrary.BreakVector` (`SceneComponent.K2_GetComponentLocation` (`self.CapsuleComponent`))))
  ;[1 1 1] Tick - Updates animation
  (if (`self.Overlapping`)
    (if (`self.AttackOverlap`)
      (set `self.Is Attacking` true)
      (else
        (bind _asbp_owlet (cast `/Game/Game/Blueprints/BP_Owlet` (`GameplayStatics.GetPlayerCharacter` 0)))
        (bind _returnvalue_x_2 (`KismetMathLibrary.BreakVector` (`SceneComponent.K2_GetComponentLocation` (`Character.CapsuleComponent` _asbp_owlet))))
        (bind _returnvalue_3 (- _returnvalue_x_2 _returnvalue_x))
        (if (<= _returnvalue_3 0.0)
          _
          (else
            _))
        (`self.AddMovementInput` (1.0 0.0 0.0) _returnvalue_3))))
  (`self.UpdateAnimation`)
  (if (`self.Is Attacking`)
    (`KismetSystemLibrary.Delay` 0.3))
  (`/Engine/EditorBlueprintResources/StandardMacros.CompareFloat` (.x (`MovementComponent.Velocity` (`self.GetMovementComponent`)))
    (:`>`
      (`/Engine/EditorBlueprintResources/StandardMacros.IsValid` _returnvalue_2 :!label _label
        (:`Is Valid`
          (`Controller.SetControlRotation` _returnvalue_2 (`KismetMathLibrary.MakeRotator` 0.0)))))
    (:`==`
      (if (`self.bisMovingRight`)
        (goto _label)
        (else
          (`/Engine/EditorBlueprintResources/StandardMacros.IsValid` _returnvalue :!label _label_2
            (:`Is Valid`
              (`Controller.SetControlRotation` _returnvalue (`KismetMathLibrary.MakeRotator` 0.0 0.0 180.0)))))))
    (:`<`
      (goto _label_2))))

(event `self.Sphere.OnComponentBeginOverlap`
  (params (OverlappedComponent :type "PrimitiveComponent Object Reference") (OtherActor :type "Actor Object Reference") (OtherComp :type "PrimitiveComponent Object Reference") (OtherBodyIndex :type Integer) (bFromSweep :type Boolean) (SweepResult :type "HitResult Structure (by ref)"))
  (cast `/Game/Game/Blueprints/BP_Owlet` OtherActor)
  (set `self.Overlapping` true))

(event `self.Sphere.OnComponentEndOverlap`
  (params (OverlappedComponent :type "PrimitiveComponent Object Reference") (OtherActor :type "Actor Object Reference") (OtherComp :type "PrimitiveComponent Object Reference") (OtherBodyIndex :type Integer))
  (cast `/Game/Game/Blueprints/BP_Owlet` OtherActor)
  (set `self.Overlapping` false))

(event `self.AttackRange.OnComponentBeginOverlap`
  (params (OverlappedComponent :type "PrimitiveComponent Object Reference") (OtherActor :type "Actor Object Reference") (OtherComp :type "PrimitiveComponent Object Reference") (OtherBodyIndex :type Integer) (bFromSweep :type Boolean) (SweepResult :type "HitResult Structure (by ref)"))
  (cast `/Game/Game/Blueprints/BP_Owlet` OtherActor)
  (set `self.AttackOverlap` true))

(fn `Animation State Machine`
  (params (IsFalling :type Boolean) (IsMoving :type Boolean) (IsRunning :type Boolean))
  (returns (OutputFlipbook :type "PaperFlipbook Object Reference"))
  (locals (`Animation State` :type "/Game/Game/Data/Character_States Enum") (IsFallingLocal :type Boolean) (IsMovingLocal :type Boolean) (IsRunningLocal :type Boolean) (IsAttackingLocal :type Boolean))
  ;[1 1 1] State Machine
  (set `local.IsFallingLocal` IsFalling)
  (set `local.IsMovingLocal` IsMoving)
  (set `local.IsRunningLocal` IsRunning)
  (set `local.IsAttackingLocal` (`self.Is Attacking`))
  (if (`local.IsAttackingLocal`)
    (set `local.Animation State` "NewEnumerator5")
    (elif (`local.IsFallingLocal`)
      (set `local.Animation State` "NewEnumerator3")
      (elif (`local.IsMovingLocal`)
        (if (`local.IsRunningLocal`)
          (set `local.Animation State` "NewEnumerator1")
          (else
            (set `local.Animation State` "NewEnumerator2")))
        (else
          (set `local.Animation State` "NewEnumerator0")))))
  (return (select `/Game/Game/Data/Character_States` (`local.Animation State`) :`NewEnumerator0` (`self.IdleFlipbook`) :`NewEnumerator2` (`self.WalkFlipbook`) :`NewEnumerator1` (`self.RunFlipbook`) :`NewEnumerator3` (`self.JumpFlipbook`))))

(fn `UserConstructionScript`)