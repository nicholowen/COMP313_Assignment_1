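; BP_Heart is a heart pickup that BP_Owlet collects on contact.
; Tick spins the PaperSprite by a fixed yaw step each frame, so spin speed depends on frame rate.
; When BP_Owlet overlaps the Sphere and its IsFull flag is false, the heart calls HeartCollect on it, plays the Heart sound and destroys itself.
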(event `self.ReceiveTick`
  (params (DeltaSeconds :type "Float (single-precision)"))
  (bind _returnvalue (`SceneComponent.GetRelativeTransform` (`self.PaperSprite`)))
  ;[1 1 1] Rotates Item
  (`SceneComponent.K2_SetWorldRotation` (`self.PaperSprite`) (`KismetMathLibrary.MakeRotator` (.roll (.rotation _returnvalue)) (.pitch (.rotation _returnvalue)) (+ (.yaw (.rotation _returnvalue)) 1.0)) false false))

(event `self.Sphere.OnComponentBeginOverlap`
  (params (OverlappedComponent :type "PrimitiveComponent Object Reference") (OtherActor :type "Actor Object Reference") (OtherComp :type "PrimitiveComponent Object Reference") (OtherBodyIndex :type Integer) (bFromSweep :type Boolean) (SweepResult :type "HitResult Structure (by ref)"))
  ;[1 1 1] Collision
  (bind _asbp_owlet (cast `/Game/Game/Blueprints/BP_Owlet` OtherActor))
  (if (not (`/Game/Game/Blueprints/BP_Owlet.IsFull` _asbp_owlet))
    (`/Game/Game/Blueprints/BP_Owlet.HeartCollect` _asbp_owlet)
    (`GameplayStatics.PlaySound2D` "/Game/Game/Sounds/heart.heart" 1.0 1.0 0.0 null null)
    (`self.K2_DestroyActor`)))

(fn `UserConstructionScript`)